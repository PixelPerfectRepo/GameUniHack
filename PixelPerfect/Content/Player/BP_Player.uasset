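; First-person player Blueprint with movement, mouse look, a toggleable cursor, weapon selection and world interaction.
; Number keys pick MathNumbers, Book or Academy; left click fires only MathNumbers when weapons are enabled, though a shorter-range Book trace exists.
; Otherwise, click traces from camera or cursor to send Interact_Interface messages, with cursor hits also grabbed by PhysicsHandle.
; Attack traces send damage through that interface, and releasing H reports an AI noise event.
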(event Custom|RayInteract
  (bind _camera (Variables|Default|GetCamera))
  (bind _returnvalue (Transformation|GetWorldLocation _camera))
  ;[1 1 1] Normal Ray Casting
  (bind (_outhit _returnvalue_2) (Collision|LineTraceByChannel _returnvalue (+ _returnvalue (* _returnvalue 1e+03)) "TraceTypeQuery1" false 0 "None"))
  (if _returnvalue_2
    (if (Utilities|DoesObjectImplementInterface (.HitActor (Collision|BreakHitResult _outhit)) "/Game/Interfaces/Interact_Interface.Interact_Interface_C")
      (Class|InteractInterface|Interact(Message) (.HitActor (Collision|BreakHitResult _outhit))))))

(event Custom|Math_Numbers
  (bind _camera (Variables|Default|GetCamera))
  (bind _returnvalue (Transformation|GetWorldLocation _camera))
  ;[1 1 1] Math Numbers Attack
  (bind (_outhit _returnvalue_2) (Collision|LineTraceByChannel _returnvalue (+ _returnvalue (* (Math|Vector|GetForwardVector _camera) 1e+03)) "TraceTypeQuery1" false 0 "ForOneFrame"))
  (if _returnvalue_2
    (if (Utilities|DoesObjectImplementInterface (.HitActor (Collision|BreakHitResult _outhit)) "/Game/Interfaces/Interact_Interface.Interact_Interface_C")
      (Class|InteractInterface|Damage(Message) (.HitActor (Collision|BreakHitResult _outhit)) 1e+02))))

(event Custom|CursorInteract
  (bind _returnvalue (Game|GetPlayerController 0))
  (bind (_worldlocation _worlddirection) (Game|Player|ConvertMouseLocationToWorldSpace _returnvalue))
  ;[1 1 1] Cursor Ray Casting
  (bind (_outhit _returnvalue_2) (Collision|LineTraceByChannel _worldlocation (+ _worldlocation (* _worlddirection 1e+03)) "TraceTypeQuery1" false 0 "ForDuration"))
  (if _returnvalue_2
    (if (Utilities|DoesObjectImplementInterface (.HitActor (Collision|BreakHitResult _outhit)) "/Game/Interfaces/Interact_Interface.Interact_Interface_C")
      (Class|InteractInterface|Interact(Message) (.HitActor (Collision|BreakHitResult _outhit)))
      (Class|PhysicsHandleComponent|GrabComponentatLocation (Variables|Default|GetPhysicsHandle) (.HitComponent (Collision|BreakHitResult _outhit)) "None" (.Location (Collision|BreakHitResult _outhit))))))

(event Custom|Book
  (bind _camera (Variables|Default|GetCamera))
  (bind _returnvalue (Transformation|GetWorldLocation _camera))
  (bind (_outhit _returnvalue_2) (Collision|LineTraceByChannel _returnvalue (+ _returnvalue (* (Math|Vector|GetForwardVector _camera) 2.5e+02)) "TraceTypeQuery1" false 0 "ForDuration"))
  (if _returnvalue_2
    (if (Utilities|DoesObjectImplementInterface (.HitActor (Collision|BreakHitResult _outhit)) "/Game/Interfaces/Interact_Interface.Interact_Interface_C")
      (Class|InteractInterface|Damage(Message) (.HitActor (Collision|BreakHitResult _outhit)) 25.0))))

(event EventPossessed
  (params (NewController :type Controller%20Object%20Reference))
  ;[1 1 1] Event Possesed
  (Input|SetInputModeGameOnly (Game|GetPlayerController 0)))

(event Input|AxisEvents|InputAxisWalkForward
  (params (AxisValue :type Float%20%28single-precision%29))
  ;[1 1 1] Movement
  (Pawn|Input|AddMovementInput (Math|Vector|GetForwardVector (Variables|Character|GetMesh)) AxisValue false))

(event Input|AxisEvents|InputAxisWalkRight
  (params (AxisValue :type Float%20%28single-precision%29))
  ;[1 1 1] Movement
  (Pawn|Input|AddMovementInput (Math|Vector|GetRightVector (Variables|Character|GetMesh)) AxisValue false))

(event Input|AxisEvents|InputAxisLookUp
  (params (AxisValue :type Float%20%28single-precision%29))
  ;[1 1 1] Look around
  (Pawn|Input|AddControllerPitchInput (* AxisValue (Variables|Default|GetSensitivity))))

(event Input|AxisEvents|InputAxisLookRight
  (params (AxisValue :type Float%20%28single-precision%29))
  ;[1 1 1] Look around
  (Pawn|Input|AddControllerYawInput (* AxisValue (Variables|Default|GetSensitivity))))

(event Input|KeyboardEvents|H
  (params (Key :type Key%20Structure :default "None"))
  (:Released
    (Class|AISenseHearing|ReportNoiseEvent (Transformation|GetActorLocation) 1.0 self 0.0 "Noise")))

(event Input|MouseEvents|LeftMouseButton
  (params (Key :type Key%20Structure :default "None"))
  ;[1 1 1] Interact
  (:Pressed
    (if (Variables|Default|GetWeapons_Enabled)
      (switch Utilities|FlowControl|Switch|SwitchonWeapons_Enum (Variables|Default|GetWeaponSeelcted)
        (:NewEnumerator0
          (CallFunction|MathNumbers)))
      (elif (not (Variables|/Script/Engine.PlayerController|GetbShowMouseCursor (Game|GetPlayerController 0)))
        (CallFunction|RayInteract)
        (else
          (CallFunction|CursorInteract))))))

(event Input|KeyboardEvents|X
  (params (Key :type Key%20Structure :default "None"))
  (bind _returnvalue (Game|GetPlayerController 0))
  ;[1 1 1] Show Cursor
  (:Pressed
    (Utilities|FlowControl|FlipFlop
      (:A
        (Variables|/Script/Engine.PlayerController|SetbShowMouseCursor _returnvalue true))
      (:B
        (Variables|/Script/Engine.PlayerController|SetbShowMouseCursor _returnvalue false)
        (Input|SetInputModeGameOnly _returnvalue)))))

(event Input|KeyboardEvents|1
  (params (Key :type Key%20Structure :default "None"))
  ;[1 1 1] Select Weapon
  (:Pressed
    (Variables|Default|SetWeaponSeelcted "NewEnumerator0")))

(event Input|KeyboardEvents|2
  (params (Key :type Key%20Structure :default "None"))
  ;[1 1 1] Select Weapon
  (:Pressed
    (Variables|Default|SetWeaponSeelcted "NewEnumerator1")))

(event Input|KeyboardEvents|3
  (params (Key :type Key%20Structure :default "None"))
  ;[1 1 1] Select Weapon
  (:Pressed
    (Variables|Default|SetWeaponSeelcted "NewEnumerator2")))

(fn ConstructionScript)